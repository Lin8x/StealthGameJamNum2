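; Interactive document item template that shows its texture on a plane and a prompt widget when something is nearby.
; A second after play begins, it creates a dynamic material from DocumentMaterial, sets DocumentTexture on it and applies it to the plane.
; Overlap with NearBox shows or hides the widget and opens or closes a Tick gate that turns it to face the player pawn.
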(event OnComponentBeginOverlap(NearBox)
  (params (OverlappedComponent :type Primitive%20Component%20Object%20Reference) (OtherActor :type Actor%20Object%20Reference) (OtherComp :type Primitive%20Component%20Object%20Reference) (OtherBodyIndex :type Integer) (bFromSweep :type Boolean) (SweepResult :type Hit%20Result%20Structure%20%28by%20ref%29))
  (Rendering|SetVisibility (Variables|Default|GetWidget) true false)
  (Utilities|FlowControl|Gate true) ; enters at Open
)

(event OnComponentEndOverlap(NearBox)
  (params (OverlappedComponent :type Primitive%20Component%20Object%20Reference) (OtherActor :type Actor%20Object%20Reference) (OtherComp :type Primitive%20Component%20Object%20Reference) (OtherBodyIndex :type Integer))
  (Rendering|SetVisibility (Variables|Default|GetWidget) false false)
  (Utilities|FlowControl|Gate true) ; enters at Close
)

(event EventBeginPlay
  (bind _plane (Variables|Default|GetPlane))
  (Rendering|SetVisibility (Variables|Default|GetWidget) false false)
  (Utilities|FlowControl|Delay 1.0)
  (bind _returnvalue (Rendering|Material|CreateDynamicMaterialInstance _plane 0 "/Game/Assets/Materials/DocumentMaterial.DocumentMaterial" "None" :!class /Script/Engine.PrimitiveComponent))
  (Rendering|Material|SetTextureParameterValue _returnvalue "Param" (Variables|Default|GetDocument%20Texture))
  (Rendering|Material|SetMaterial _plane 0 _returnvalue))

(event EventTick
  (params (DeltaSeconds :type Float%20%28single-precision%29))
  (Utilities|FlowControl|Gate true
    (:Exit
      (Transformation|SetWorldRotation (Variables|Default|GetWidget) (Math|Rotator|FindLookatRotation (Transformation|GetWorldLocation (Variables|Default|GetWidget)) (Transformation|GetActorLocation (Game|Player|GetPlayerPawn 0))) false false))))

(fn ConstructionScript)