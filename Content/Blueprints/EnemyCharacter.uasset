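; Zombie enemy character that wanders, chases and kills the player, and can be stabbed at a weak point.
; Tick starts random navmesh roaming with look-around pauses, while pawn sensing triggers a faster run to the player's last location.
; Mutually exclusive animation booleans act as the state, switching speed and sounds.
; AttackArea overlaps call CharDie on the player; stabbing inside WeakPoint destroys the zombie and updates the player's kill counter.
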(event OnSeePawn(PawnSensing)
  (params (Pawn :type Pawn%20Object%20Reference))
  (bind _zombiesoundlocation (Variables|Default|GetZombieSoundLocation))
  (if (not (Variables|Default|GetAttackAnimation))
    (bind _ascharacter_player (Utilities|Casting|CastToCharacterPlayer (Game|GetPlayerCharacter 0)))
    (Development|PrintString "FOUND YOU" true true "(R=1.000000,G=0.000000,B=0.089443,A=1.000000)")
    (if (Audio|Components|Audio|IsPlaying _zombiesoundlocation)
      _
      (else
        (Audio|Components|Audio|SetSound _zombiesoundlocation "/Game/Assets/Audio/Cues/ZombieChaseScreamNoBegEnd_Cue.ZombieChaseScreamNoBegEnd_Cue")
        (Audio|Components|Audio|Play _zombiesoundlocation 0.0)))
    (CallFunction|Run)
    (AI|AIMoveTo self (Class|CharacterMovementComponent|GetLastUpdateLocation (Variables|/Script/Engine.Character|GetCharacterMovement _ascharacter_player)) 0 5.0 false
      (:OnSuccess
        (Audio|Components|Audio|FadeOut (Variables|Default|GetZombieSoundLocation) 1.0 0.0 "Linear" :!class /Script/Engine.AudioComponent)
        (CallFunction|LookAround))
      (:OnFail
        (Development|PrintString "FAILED" true true "(R=1.000000,G=0.069327,B=0.000000,A=1.000000)")))))

(event OnComponentBeginOverlap(AttackArea)
  (params (OverlappedComponent :type Primitive%20Component%20Object%20Reference) (OtherActor :type Actor%20Object%20Reference) (OtherComp :type Primitive%20Component%20Object%20Reference) (OtherBodyIndex :type Integer) (bFromSweep :type Boolean) (SweepResult :type Hit%20Result%20Structure%20%28by%20ref%29))
  (bind _ascharacter_player (Utilities|Casting|CastToCharacterPlayer OtherActor))
  (if (Utilities|IsValid _ascharacter_player)
    (if (not (Variables|Default|GetAttackAnimation))
      (Variables|Default|SetWalkAnimation false)
      (Variables|Default|SetisRunning false)
      (Variables|Default|SetLookAroundAnimation false)
      (Variables|Default|SetAttackAnimation true)
      (Utilities|FlowControl|Delay 0.4)
      (Default|CharDie _ascharacter_player))))

(event OnComponentEndOverlap(AttackArea)
  (params (OverlappedComponent :type Primitive%20Component%20Object%20Reference) (OtherActor :type Actor%20Object%20Reference) (OtherComp :type Primitive%20Component%20Object%20Reference) (OtherBodyIndex :type Integer))
  (bind _ascharacter_player (Utilities|Casting|CastToCharacterPlayer (stale OnComponentBeginOverlap(AttackArea) OtherActor)))
  (if (Utilities|IsValid _ascharacter_player)
    (if (not (Variables|Default|GetAttackAnimation))
      (Variables|Default|SetWalkAnimation false)
      (Variables|Default|SetisRunning false)
      (Variables|Default|SetLookAroundAnimation false)
      (Variables|Default|SetAttackAnimation true)
      (Utilities|FlowControl|Delay 0.4)
      (Default|CharDie _ascharacter_player))))

(event OnComponentBeginOverlap(WeakPoint)
  (params (OverlappedComponent :type Primitive%20Component%20Object%20Reference) (OtherActor :type Actor%20Object%20Reference) (OtherComp :type Primitive%20Component%20Object%20Reference) (OtherBodyIndex :type Integer) (bFromSweep :type Boolean) (SweepResult :type Hit%20Result%20Structure%20%28by%20ref%29))
  (bind _ascharacter_player (Utilities|Casting|CastToCharacterPlayer OtherActor))
  (Variables|Default|SetAs%20Character%20Player _ascharacter_player)
  (Variables|Default|SetdeathReady true))

(event OnComponentEndOverlap(WeakPoint)
  (params (OverlappedComponent :type Primitive%20Component%20Object%20Reference) (OtherActor :type Actor%20Object%20Reference) (OtherComp :type Primitive%20Component%20Object%20Reference) (OtherBodyIndex :type Integer))
  (Utilities|Casting|CastToCharacterPlayer OtherActor)
  (Variables|Default|SetdeathReady false))

(event Custom|Attack
  (Variables|Default|SetLookAroundAnimation false)
  (Variables|Default|SetisRunning false)
  (Variables|Default|SetWalkAnimation false)
  (Variables|Default|SetAttackAnimation true))

(event Custom|Run
  (if (not (Variables|Default|GetAttackAnimation))
    (Variables|Default|SetisRunning true)
    (Variables|Default|SetLookAroundAnimation false)
    (Variables|Default|SetAttackAnimation false)
    (Variables|Default|SetWalkAnimation false)
    (Variables|/Script/Engine.CharacterMovementComponent|SetMaxWalkSpeed (Variables|Character|GetCharacterMovement) 2.5e+02)))

(event Custom|Walk
  (bind _zombiesoundlocation (Variables|Default|GetZombieSoundLocation))
  (if (not (Variables|Default|GetisRunning))
    (Variables|/Script/Engine.CharacterMovementComponent|SetMaxWalkSpeed (Variables|Character|GetCharacterMovement) 1e+02)
    (if (Audio|Components|Audio|IsPlaying _zombiesoundlocation)
      _
      (else
        (Audio|Components|Audio|SetSound _zombiesoundlocation "/Game/Assets/Audio/Cues/ZombieMoanRandom.ZombieMoanRandom")
        (Audio|Components|Audio|Play _zombiesoundlocation 0.0)))
    (Variables|Default|SetLookAroundAnimation false)
    (Variables|Default|SetAttackAnimation false)
    (Variables|Default|SetisRunning false)
    (Variables|Default|SetWalkAnimation true)))

(event Custom|LookAround
  (Development|PrintString "Look Around" true true "(R=1.000000,G=0.000000,B=0.856692,A=1.000000)")
  (Variables|Default|SetWalkAnimation false)
  (Variables|Default|SetAttackAnimation false)
  (Variables|Default|SetisRunning false)
  (Variables|Default|SetLookAroundAnimation true)
  (Utilities|FlowControl|Delay 1e+01)
  (Variables|Default|SetLookAroundAnimation false))

(event EventBeginPlay
  (bind _ascharacter_player (Utilities|Casting|CastToCharacterPlayer (Game|Player|GetPlayerPawn 0)))
  (Variables|Default|SetAs%20Character%20Player _ascharacter_player)
  (Utilities|FlowControl|Delay 0.2)
  (Variables|/Game/Blueprints/CharacterPlayer.CharacterPlayer_C|SetTotalEnemies _ascharacter_player (+ (Variables|/Game/Blueprints/CharacterPlayer.CharacterPlayer_C|GetTotalEnemies _ascharacter_player) 1))
  (Variables|/Game/Blueprints/CharacterPlayer.CharacterPlayer_C|SetEnemiesToKill _ascharacter_player 0))

(event Collision|EventActorBeginOverlap
  (params (OtherActor :type Actor%20Object%20Reference)))

(event EventTick
  (params (DeltaSeconds :type Float%20%28single-precision%29))
  (bind _self self)
  (bind _as_character_player (Variables|Default|GetAs%20Character%20Player))
  (bind _zombiesoundlocation (Variables|Default|GetZombieSoundLocation))
  (Variables|Default|SetCharSpeed (Math|Vector|VectorLength (Transformation|GetVelocity)))
  (Utilities|FlowControl|Sequence
    (:then_0
      (if (not (Variables|Default|GetWalkAnimation))
        (if (not (Variables|Default|GetisRunning))
          (if (not (Variables|Default|GetLookAroundAnimation))
            (if (not (Variables|Default|GetAttackAnimation))
              (CallFunction|Walk)
              (AI|AIMoveTo _self (.RandomLocation (Class|NavigationSystemV1|GetRandomPointinNavigableRadius (Transformation|GetActorLocation _self) 2e+03 0 0)) 0 5.0 true
                (:OnSuccess
                  (CallFunction|LookAround))))))))
    (:then_1
      (if (Variables|Default|GetdeathReady)
        (if (Variables|/Game/Blueprints/CharacterPlayer.CharacterPlayer_C|GetstabbingAnimation (Variables|Default|GetAs%20Character%20Player))
          (Components|Movement|StopMovementImmediately (Variables|Character|GetCharacterMovement))
          (CallFunction|LookAround)
          (Input|SetIgnoreMoveInput (Pawn|GetController self) false)
          (Audio|Components|Audio|SetSound _zombiesoundlocation "/Game/Assets/Audio/Cues/ZombieInPain_Cue.ZombieInPain_Cue")
          (Audio|Components|Audio|Play _zombiesoundlocation 0.0)
          (Audio|Components|Audio|FadeOut _zombiesoundlocation 2.0 0.0 "Linear" :!class /Script/Engine.AudioComponent)
          (Utilities|FlowControl|Delay 2.0)
          (if (not (Variables|Default|GetdeathAnimation))
            (Variables|Default|SetdeathAnimation true)
            (Utilities|FlowControl|Delay 1.0)
            (if (!= (Variables|/Game/Blueprints/CharacterPlayer.CharacterPlayer_C|GetEnemiesToKill _as_character_player) (Variables|/Game/Blueprints/CharacterPlayer.CharacterPlayer_C|GetTotalEnemies _as_character_player))
              (Variables|/Game/Blueprints/CharacterPlayer.CharacterPlayer_C|SetEnemiesToKill _as_character_player (+ (Variables|/Game/Blueprints/CharacterPlayer.CharacterPlayer_C|GetEnemiesToKill _as_character_player) 1))
              (Actor|DestroyActor))))))))

(fn ConstructionScript)